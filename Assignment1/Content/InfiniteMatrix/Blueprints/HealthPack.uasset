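; Health pickup actor that spins slightly every Tick and adds a fixed amount of health to BP_Player on contact.
; Overlap and hit events on both the mesh and collision components share one path that casts to BP_Player and increases Health without clamping.
; If the HealthPack reference is valid, it then destroys only the mesh component, leaving the actor and collision component in place.
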(event OnComponentBeginOverlap(HealthPackMesh)
  (params (OverlappedComponent :type Primitive%20Component%20Object%20Reference) (OtherActor :type Actor%20Object%20Reference) (OtherComp :type Primitive%20Component%20Object%20Reference) (OtherBodyIndex :type Integer) (bFromSweep :type Boolean) (SweepResult :type Hit%20Result%20Structure%20%28by%20ref%29))
  (bind _asbp_player (Utilities|Casting|CastToBP_Player (stale OnComponentHit(HealthPackCollision) OtherActor)))
  (Variables|/Game/InfiniteMatrix/Blueprints/BP_Player.BP_Player_C|SetHealth _asbp_player (+ 3e+01 (Variables|/Game/InfiniteMatrix/Blueprints/BP_Player.BP_Player_C|GetHealth _asbp_player)))
  (if (Utilities|IsValid "HealthPack")
    (Utilities|FlowControl|Sequence
      (:then_0
        (Components|DestroyComponent (Variables|Default|GetHealthPackMesh))))))

(event OnComponentHit(HealthPackMesh)
  (params (HitComponent :type Primitive%20Component%20Object%20Reference) (OtherActor :type Actor%20Object%20Reference) (OtherComp :type Primitive%20Component%20Object%20Reference) (NormalImpulse :type Vector :default "0, 0, 0") (Hit :type Hit%20Result%20Structure%20%28by%20ref%29))
  (bind _asbp_player (Utilities|Casting|CastToBP_Player (stale OnComponentHit(HealthPackCollision) OtherActor)))
  (Variables|/Game/InfiniteMatrix/Blueprints/BP_Player.BP_Player_C|SetHealth _asbp_player (+ 3e+01 (Variables|/Game/InfiniteMatrix/Blueprints/BP_Player.BP_Player_C|GetHealth _asbp_player)))
  (if (Utilities|IsValid "HealthPack")
    (Utilities|FlowControl|Sequence
      (:then_0
        (Components|DestroyComponent (Variables|Default|GetHealthPackMesh))))))

(event OnComponentBeginOverlap(HealthPackCollision)
  (params (OverlappedComponent :type Primitive%20Component%20Object%20Reference) (OtherActor :type Actor%20Object%20Reference) (OtherComp :type Primitive%20Component%20Object%20Reference) (OtherBodyIndex :type Integer) (bFromSweep :type Boolean) (SweepResult :type Hit%20Result%20Structure%20%28by%20ref%29))
  (bind _asbp_player (Utilities|Casting|CastToBP_Player (stale OnComponentHit(HealthPackCollision) OtherActor)))
  (Variables|/Game/InfiniteMatrix/Blueprints/BP_Player.BP_Player_C|SetHealth _asbp_player (+ 3e+01 (Variables|/Game/InfiniteMatrix/Blueprints/BP_Player.BP_Player_C|GetHealth _asbp_player)))
  (if (Utilities|IsValid "HealthPack")
    (Utilities|FlowControl|Sequence
      (:then_0
        (Components|DestroyComponent (Variables|Default|GetHealthPackMesh))))))

(event OnComponentHit(HealthPackCollision)
  (params (HitComponent :type Primitive%20Component%20Object%20Reference) (OtherActor :type Actor%20Object%20Reference) (OtherComp :type Primitive%20Component%20Object%20Reference) (NormalImpulse :type Vector :default "0, 0, 0") (Hit :type Hit%20Result%20Structure%20%28by%20ref%29))
  (bind _asbp_player (Utilities|Casting|CastToBP_Player OtherActor))
  (Variables|/Game/InfiniteMatrix/Blueprints/BP_Player.BP_Player_C|SetHealth _asbp_player (+ 3e+01 (Variables|/Game/InfiniteMatrix/Blueprints/BP_Player.BP_Player_C|GetHealth _asbp_player)))
  (if (Utilities|IsValid "HealthPack")
    (Utilities|FlowControl|Sequence
      (:then_0
        (Components|DestroyComponent (Variables|Default|GetHealthPackMesh))))))

(event EventBeginPlay)

(event Collision|EventActorBeginOverlap
  (params (OtherActor :type Actor%20Object%20Reference)))

(event EventTick
  (params (DeltaSeconds :type Float%20%28single-precision%29))
  (Transformation|AddActorLocalRotation "0.000000,2.000000,0.000000" false false))

(fn ConstructionScript)